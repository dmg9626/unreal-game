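; An actor that each tick orbits an optional TargetActor and spins itself, each around its own axis and degrees-per-second rate.
; RevolveAroundTarget rotates the offset from the target and repositions the actor without sweeping, only while the target is valid.
; RotateSelf rotates the forward vector and rebuilds rotation from that direction alone.
; The construction script caches a MovingGrappleComponent reference if unset, though these graphs never use it further.
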(event `self.ReceiveTick`
  (params (DeltaSeconds :type "Float (single-precision)"))
  (bind _returnvalue (`self.K2_GetActorLocation` (`self.TargetActor`)))
  (`|ExecutionSequence`
    (:`then_0`
      (`/Engine/EditorBlueprintResources/StandardMacros.IsValid` (`self.TargetActor`)
        (:`Is Valid`
          (`self.K2_SetActorLocation` (+ _returnvalue (`KismetMathLibrary.RotateAngleAxis` (- (`self.K2_GetActorLocation`) _returnvalue) (* DeltaSeconds (`self.Revolve_DegreesPerSecond`)) (`self.RevolveAxis`)))))))
    (:`then_1`
      (`self.K2_SetActorRotation` (`KismetMathLibrary.Quat_Rotator` (`KismetMathLibrary.Conv_VectorToQuaterion` (`KismetMathLibrary.RotateAngleAxis` (`self.GetActorForwardVector`) (* DeltaSeconds (`self.Rotate_DegreesPerSecond`)) (`self.RotateAxis`))))))))

(fn `UserConstructionScript`
  (`/Engine/EditorBlueprintResources/StandardMacros.IsValid` (`self.MovingGrapple`)
    (:`Is Not Valid`
      (set `self.MovingGrapple` (`self.GetComponentByClass` "/Script/UnrealProject.MovingGrappleComponent")))))