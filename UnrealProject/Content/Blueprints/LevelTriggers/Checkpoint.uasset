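; Checkpoint trigger actor that records itself as the active checkpoint when the player character overlaps it.
; On BeginPlay it caches the FirstPersonGameMode, printing an error if the cast fails.
; Overlaps by a GrappleCharacter_Redux pass the checkpoint to the game mode through SetCheckpoint.
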(event `self.ReceiveBeginPlay`
  ;[1 1 1] Store reference to game mode
  (bind _asfirst_person_game_mode (cast `/Game/FirstPersonBP/Blueprints/FirstPersonGameMode` (`GameplayStatics.GetGameMode`))
    (:`then`
      (set `self.FirstPersonGameMode` _asfirst_person_game_mode))
    (:`CastFailed`
      (`KismetSystemLibrary.PrintString` "ERROR - failed to cast game mode to FirstPersonGameMode" true true (struct :`G` 0.66 :`B` 1.0 :`A` 1.0) 5.0))))

(event `self.ReceiveActorBeginOverlap`
  (params (OtherActor :type "Actor Object Reference"))
  (cast `/Game/Blueprints/Player/GrappleCharacter_Redux` OtherActor)
  (`/Game/FirstPersonBP/Blueprints/FirstPersonGameMode.SetCheckpoint` (`self.FirstPersonGameMode`) self))

(fn `UserConstructionScript`)