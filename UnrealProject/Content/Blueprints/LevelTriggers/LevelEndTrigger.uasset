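; Level-end trigger actor that signals level completion when the player reaches it and can load the next level.
; On BeginPlay it caches the FirstPersonGameMode, printing an error if the cast fails.
; Overlap by the player character calls OnLevelComplete on the game mode, passing itself.
; Its LoadNextLevel event hides the cursor, restores game-only input and opens the level named by NextLevel.
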(event `self.ReceiveBeginPlay`
  (bind _asfirst_person_game_mode (cast `/Game/FirstPersonBP/Blueprints/FirstPersonGameMode` (`GameplayStatics.GetGameMode`))
    (:`then`
      (set `self.GameMode` _asfirst_person_game_mode))
    (:`CastFailed`
      (`KismetSystemLibrary.PrintString` "ERROR - failed to cast game mode to FirstPersonGameMode" true true (struct :`G` 0.66 :`B` 1.0 :`A` 1.0) 5.0))))

(event `self.ReceiveActorBeginOverlap`
  (params (OtherActor :type "Actor Object Reference"))
  ;[1 1 1] Detect when player reaches end of level
  (if (== OtherActor (`GameplayStatics.GetPlayerCharacter` 0))
    (`/Game/FirstPersonBP/Blueprints/FirstPersonGameMode.On Level Complete` (`self.GameMode`) self) ; Trigger level complete sequence \nin game mode blueprint
  ))

(event `Load Next Level`
  (bind _returnvalue (`GameplayStatics.GetPlayerController` 0))
  ;[1 1 1] Load Next Level
  (set `PlayerController.bShowMouseCursor` false _returnvalue) ; Hide mouse cursor
  (`WidgetBlueprintLibrary.SetInputMode_GameOnly` _returnvalue) ; Restore input control to game
  (`GameplayStatics.OpenLevel` (`self.NextLevel`)))

(fn `UserConstructionScript`)