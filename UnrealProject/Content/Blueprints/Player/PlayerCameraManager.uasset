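; Player camera manager that widens the field of view as the player pawn moves faster.
; BeginPlay caches player 0's pawn and starts the current FOV at the base value.
; Each Tick derives a target FOV from base plus velocity magnitude over a scalar, then eases DefaultFOV toward it by a fixed fraction per frame, without delta-time scaling.
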(event `self.ReceiveBeginPlay`
  (set `self.Player` (`GameplayStatics.GetPlayerPawn` 0))
  (set `self.CurrentFov` (`self.BaseFov`)))

(event `self.ReceiveTick`
  (params (DeltaSeconds :type "Float (single-precision)"))
  (bind _currentfov (`self.CurrentFov`))
  ;[1 1 1] Scale FOV By Speed
  (bind _output_get (set `self.TargetFov` (+ (`self.BaseFov`) (/ (`KismetMathLibrary.VSize` (`self.GetVelocity` (`self.Player`))) (`self.SpeedToFovScalar`)))))
  (bind _output_get_2 (set `self.CurrentFov` (+ (* (- _output_get _currentfov) (`self.FovStep`)) _currentfov)))
  (set `self.DefaultFOV` _output_get_2))

(fn `UserConstructionScript`)